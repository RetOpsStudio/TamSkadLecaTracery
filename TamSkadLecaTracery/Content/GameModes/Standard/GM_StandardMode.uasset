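; Standard game mode Blueprint that tracks a ticket count for the Green and Red teams.
; The construction script gives both teams the same starting ticket count.
; IncreaseTickets and DecreaseTickets switch on a team index, 0 for Green and 1 for Red, to adjust that team's total.
; It applies no clamping or win check, and its event graph is empty.
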(event EventBeginPlay)

(event EventTick
  (params (DeltaSeconds :type Float%20%28single-precision%29)))

(fn ConstructionScript
  ;[1 1 1] set starting tickets
  (Variables|Default|SetGreenTeamTickets 10)
  (Variables|Default|SetRedTeamTickets 10))

(fn IncreaseTickets
  (params (IncreaseAmount :type Integer) (Team :type Integer))
  (switch int Team
    (:0
      ;[1 1 1] green alias  0
      (Variables|Default|SetGreenTeamTickets (+ (Variables|Default|GetGreenTeamTickets) IncreaseAmount)))
    (:1
      ;[1 1 1] red alias 1
      (Variables|Default|SetRedTeamTickets (+ (Variables|Default|GetRedTeamTickets) IncreaseAmount)))))

(fn DecreaseTickets
  (params (DecreaseAmount :type Integer) (Team :type Integer))
  (switch int Team
    (:0
      ;[1 1 1] green alias  0
      (Variables|Default|SetGreenTeamTickets (- (Variables|Default|GetGreenTeamTickets) DecreaseAmount)))
    (:1
      ;[1 1 1] red alias 1
      (Variables|Default|SetRedTeamTickets (- (Variables|Default|GetRedTeamTickets) DecreaseAmount)))))