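; Player character Blueprint for a shooter with switchable first/third-person cameras, movement, a gun and death.
; Input drives movement and a child-actor BP_GunBase, pushing state to ABP_PlayerCharacter and the HUD.
; Looping timers interpolate camera switches and aim-down-sights, and back the character away when its head overlaps walls.
; Data tables configure speeds, per-limb hitboxes and gun animation values; lethal damage triggers ragdoll and interface-based kill/death messages.
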(event EventBeginPlay
  (bind _abpinstance (Variables|References|GetABPInstance))
  (Setup|GetABPReference)
  (Class|DefaultCH|SetupVariables (Variables|References|GetABPInstance))
  (Variables|/Game/Characters/Player/ABP_PlayerCharacter.ABP_PlayerCharacter_C|SetDiff _abpinstance (+ (.yaw (Variables|/Game/Characters/Player/ABP_PlayerCharacter.ABP_PlayerCharacter_C|GetUpperSpineRotation _abpinstance)) 9e+01))
  (Utilities|FlowControl|Delay 0.1)
  ;[1 1 1] Setup Gun
  (ChildActorComponent|SetChildActorClass (Variables|Default|GetPrimaryWeapon) (Variables|Default|GetStartingWeapon))
  (Weapon|SetPrimaryWActorRef)
  (Variables|/Game/Guns/BP_Guns/BP_GunBase.BP_GunBase_C|SetControllerRef (Variables|References|GetPrimaryWActorRef) (Components|GetOwner))
  (Utilities|FlowControl|Delay 0.1)
  (Setup|SetupGunVariablesinABP)
  (CallFunction|SwitchCamtoFpsEvent)
  ;[1 1 1] prevents "access none"
  (Utilities|Casting|CastToPlayerController (Components|GetOwner self))
  (Weapon|UpdateAmmo)
  ;[1 1 1] setting up player controllerId variable
  (bind _asplayer_controller (Utilities|Casting|CastToPlayerController (Components|GetOwner)))
  (bind _output_get (Variables|Default|SetPlayerControllerID (Class|GameplayStatics|GetPlayerControllerID _asplayer_controller)))
  (Variables|/Game/Guns/BP_Guns/BP_GunBase.BP_GunBase_C|SetPlayerControllerID (Variables|References|GetPrimaryWActorRef) _output_get))

(event Collision|EventActorBeginOverlap
  (params (OtherActor :type Actor%20Object%20Reference)))

(event OnComponentBeginOverlap(Head)
  (params (OverlappedComponent :type Primitive%20Component%20Object%20Reference) (OtherActor :type Actor%20Object%20Reference) (OtherComp :type Primitive%20Component%20Object%20Reference) (OtherBodyIndex :type Integer) (bFromSweep :type Boolean) (SweepResult :type Hit%20Result%20Structure%20%28by%20ref%29))
  ;[1 1 1] prevents putting head inside a wall
  (Utilities|Casting|CastToBP_PlayerCH OtherActor
    (:CastFailed
      (Utilities|Casting|CastToBP_GunBase OtherActor
        (:CastFailed
          (bind _returnvalue (Utilities|Time|SetTimerbyFunctionName 0 "MoveOutOfTheWall" (Utilities|Time|GetWorldDeltaSeconds) true)))))))

(event OnComponentEndOverlap(Head)
  (params (OverlappedComponent :type Primitive%20Component%20Object%20Reference) (OtherActor :type Actor%20Object%20Reference) (OtherComp :type Primitive%20Component%20Object%20Reference) (OtherBodyIndex :type Integer))
  ;[1 1 1] prevents putting head inside a wall
  (Utilities|Casting|CastToBP_PlayerCH OtherActor
    (:CastFailed
      (Utilities|Casting|CastToBP_GunBase OtherActor
        (:CastFailed
          (Utilities|Time|ClearandInvalidateTimerbyHandle (stale OnComponentBeginOverlap(Head) _returnvalue)))))))

(event Custom|SwitchCam_Event
  (bind _tpcamera (Variables|Default|GetTPCamera))
  (bind _returnvalue (Transformation|GetWorldLocation _tpcamera))
  ;[1 1 1] FULL PROTOTYPE SMOOTH CAMERA SQITCH
  ;;[1 1 1] Interp to TPS Camera
  (bind _returnvalue_2 (Utilities|Time|SetTimerbyEvent (delegate Custom|SwitchCam_Event) (/ (Utilities|Time|GetWorldDeltaSeconds) 2.0) true))
  (Utility|ChangeCam _returnvalue 25.0)
  (if (Math|Vector|Equal(Vector) _returnvalue (Transformation|GetWorldLocation (Variables|Default|GetFPCamera)) 1e+02)
    (Utilities|Time|ClearandInvalidateTimerbyHandle _returnvalue_2)
    (Components|Activation|ToggleActive (Variables|Default|GetFPCamera))
    (Components|Activation|ToggleActive (Variables|Default|GetTPCamera))))

(event Custom|SwitchCamToFps_Event
  (bind _fpcameraslot (Variables|Default|GetFPCameraSlot))
  (bind _returnvalue (Transformation|GetWorldLocation _fpcameraslot))
  ;[1 1 1] FULL PROTOTYPE SMOOTH CAMERA SQITCH
  ;;[1 1 1] Go Back To FPS CAMERA
  (bind _returnvalue_2 (Utilities|Time|SetTimerbyEvent (delegate Custom|SwitchCamToFps_Event) (/ (Utilities|Time|GetWorldDeltaSeconds) 2.0) true))
  (Utility|ChangeCam _returnvalue 2e+01)
  (if (Math|Vector|Equal(Vector) _returnvalue (Transformation|GetWorldLocation (Variables|Default|GetFPCamera)) 0.1)
    (Utilities|Time|ClearandInvalidateTimerbyHandle _returnvalue_2)
    (Variables|UtilytyBooleans|Setb_IsTps false)))

(event EventTick
  (params (DeltaSeconds :type Float%20%28single-precision%29))
  (bind _abpinstance (Variables|References|GetABPInstance))
  (bind _diff (Variables|/Game/Characters/Player/ABP_PlayerCharacter.ABP_PlayerCharacter_C|GetDiff _abpinstance))
  ;[1 1 1] (legs rotation over time) sphagetti intensifies
  (Variables|/Game/Characters/Player/ABP_PlayerCharacter.ABP_PlayerCharacter_C|SetNewRot _abpinstance (.yaw (Math|Interpolation|RInterpTo (Math|Rotator|MakeRotator 0.0 0.0 (Variables|/Game/Characters/Player/ABP_PlayerCharacter.ABP_PlayerCharacter_C|GetNewRot _abpinstance)) (Math|Rotator|MakeRotator 0.0 0.0 _diff) DeltaSeconds (Math|Float|Clamp(Float) (* 15 (- 1.0 (Math|Vector|DotProduct (Math|Vector|GetForwardVector (Math|Rotator|MakeRotator 0.0 0.0 (Variables|/Game/Characters/Player/ABP_PlayerCharacter.ABP_PlayerCharacter_C|GetNewRot _abpinstance))) (Math|Vector|GetForwardVector (Math|Rotator|MakeRotator 0.0 0.0 _diff))))) 4.0 999.0)))))

(event Input|ActionEvents|InputActionJump
  (params (Key :type Key%20Structure))
  (bind _abpinstance (Variables|References|GetABPInstance))
  ;[1 1 1] Movement
  ;;[1 1 1] Jumping
  (:Pressed
    (Variables|/Game/Characters/Player/ABP_PlayerCharacter.ABP_PlayerCharacter_C|SetEnable%20Jump _abpinstance (not (Variables|/Game/Characters/Player/ABP_PlayerCharacter.ABP_PlayerCharacter_C|GetEnable%20Jump _abpinstance)))
    (Character|Jump)
    (Utilities|FlowControl|Delay 0.1)
    (Variables|/Game/Characters/Player/ABP_PlayerCharacter.ABP_PlayerCharacter_C|SetEnable%20Jump _abpinstance (not (Variables|/Game/Characters/Player/ABP_PlayerCharacter.ABP_PlayerCharacter_C|GetEnable%20Jump _abpinstance)))))

(event Input|ActionEvents|InputActionCrouch
  (params (Key :type Key%20Structure))
  (bind _capsulecomponent (Variables|Default|GetCapsuleComponent))
  (bind _abpinstance (Variables|References|GetABPInstance))
  (bind _returnvalue (Physics|GetCenterOfMass _capsulecomponent "None"))
  (bind _returnvalue_2 (+ (.z _returnvalue) 5e+01))
  ;[1 1 1] Movement
  ;;[1 1 1] Crouching
  (:Pressed
    (if (not (Variables|/Game/Characters/Player/ABP_PlayerCharacter.ABP_PlayerCharacter_C|GetCrouching _abpinstance))
      (Variables|/Game/Characters/Player/ABP_PlayerCharacter.ABP_PlayerCharacter_C|SetCrouching _abpinstance (not (Variables|/Game/Characters/Player/ABP_PlayerCharacter.ABP_PlayerCharacter_C|GetCrouching _abpinstance)) :!label _label)
      (Utilities|FlowControl|FlipFlop
        (:A
          (Character|Crouch))
        (:B
          (Character|UnCrouch)))
      (else
        ;[1 1 1] checks if CH can stand without head colision
        (bind _returnvalue_3 (Collision|CapsuleTraceByChannel (Math|Vector|MakeVector (.x _returnvalue) (.y _returnvalue) _returnvalue_2) (Math|Vector|MakeVector (.x _returnvalue) (.y _returnvalue) _returnvalue_2) (- (Variables|/Script/Engine.CapsuleComponent|GetCapsuleRadius _capsulecomponent) 11.0) 88.0 "TraceTypeQuery1" false 0 "None"))
        (if (not _returnvalue_3)
          (goto _label)
          (else
            (Default|ShowTipsEvent (Variables|References|GetHud))))))))

(event Input|ActionEvents|InputActionCameraSwitch
  (params (Key :type Key%20Structure))
  ;[1 1 1] FULL PROTOTYPE SMOOTH CAMERA SQITCH
  (:Pressed
    (if (and (not (or (Utilities|Time|IsTimerActivebyHandle (stale Custom|SwitchCam_Event _returnvalue_2)) (Utilities|Time|IsTimerActivebyHandle (stale Custom|SwitchCamToFps_Event _returnvalue_2)))) (not (Variables|UtilytyBooleans|Getb_AimingDownSights)))
      (Utilities|FlowControl|FlipFlop
        (:A
          ;;[1 1 1] to TPS
          (Variables|/Script/Engine.CameraComponent|SetbUsePawnControlRotation (Variables|Default|GetFPCamera) false)
          (CallFunction|SwitchCamEvent)
          (Variables|UtilytyBooleans|Setb_IsTps true))
        (:B
          ;;[1 1 1] to FPS
          (CallFunction|SwitchCamtoFpsEvent)
          (Components|Activation|ToggleActive (Variables|Default|GetFPCamera))
          (Components|Activation|ToggleActive (Variables|Default|GetTPCamera))
          (Variables|/Script/Engine.CameraComponent|SetbUsePawnControlRotation (Variables|Default|GetFPCamera) true))))))

(event Input|ActionEvents|InputActionwalk
  (params (Key :type Key%20Structure))
  (bind _charactermovement (Variables|Character|GetCharacterMovement))
  ;[1 1 1] Movement
  ;;[1 1 1] Walking
  (:Pressed
    (Variables|/Script/Engine.CharacterMovementComponent|SetMaxWalkSpeed _charactermovement (Variables|Movement|GetWalkSpeed))
    (Variables|UtilytyBooleans|Setb_IsWalking true))
  (:Released
    (if (not (Variables|UtilytyBooleans|Getb_AimingDownSights))
      (Variables|/Script/Engine.CharacterMovementComponent|SetMaxWalkSpeed _charactermovement (Variables|Movement|GetJogSpeed)))
    (Variables|UtilytyBooleans|Setb_IsWalking false)))

(event Input|AxisEvents|InputAxisMovCamY
  (params (AxisValue :type Float%20%28single-precision%29))
  (bind _returnvalue (Pawn|GetControlRotation :!class /Script/Engine.Pawn))
  ;[1 1 1] RotationXY
  (Pawn|Input|AddControllerPitchInput (* -1 AxisValue))
  ;[1 1 1] Switch Camera
  ;;[1 1 1] 3PS SpringArm rotation
  (Transformation|SetRelativeRotation (Variables|Default|GetSpringArm) (Math|Rotator|MakeRotator (.roll _returnvalue) (.pitch _returnvalue) (- (.yaw _returnvalue) 9e+01)) false false))

(event Input|AxisEvents|InputAxisMovForwardBackward
  (params (AxisValue :type Float%20%28single-precision%29))
  ;[1 1 1] Movement
  ;;[1 1 1] WSAD
  (Pawn|Input|AddMovementInput (Math|Vector|GetForwardVector (Math|Rotator|MakeRotator 0.0 0.0 (.yaw (Pawn|GetControlRotation :!class /Script/Engine.Pawn)))) (Math|Float|Sign(Float) AxisValue) false)
  ;;[1 1 1] Calc and sed direction in ABP
  (Setup|SetSpeedandDirection))

(event Input|AxisEvents|InputAxisMovLeftRight
  (params (AxisValue :type Float%20%28single-precision%29))
  ;[1 1 1] Movement
  ;;[1 1 1] WSAD
  (Pawn|Input|AddMovementInput (Math|Vector|GetRightVector (Math|Rotator|MakeRotator 0.0 0.0 (.yaw (Pawn|GetControlRotation :!class /Script/Engine.Pawn)))) AxisValue false)
  ;;[1 1 1] Calc and sed direction in ABP
  (Setup|SetSpeedandDirection))

(event Input|AxisEvents|InputAxisMovCamX
  (params (AxisValue :type Float%20%28single-precision%29))
  (bind _abpinstance (Variables|References|GetABPInstance))
  ;[1 1 1] RotationXY
  (Variables|Default|SetCameraDeltaRotationX AxisValue)
  ;;[1 1 1] if more then X degree
  (bind _output_get (Variables|Movement|SetRotation (+ (Variables|Movement|GetRotation) (Variables|Default|GetCameraDeltaRotationX))))
  ;[1 1 1] move spine
  (Default|ItsMeDio (Variables|References|GetABPInstance))
  (Pawn|Input|AddControllerYawInput (Variables|Default|GetCameraDeltaRotationX))
  (if (or (> (Math|Float|Absolute(Float) _output_get) 2e+01) (> (Variables|/Game/Characters/Player/ABP_PlayerCharacter.ABP_PlayerCharacter_C|GetSpeed _abpinstance) 1.0))
    (Variables|/Game/Characters/Player/ABP_PlayerCharacter.ABP_PlayerCharacter_C|SetRotate _abpinstance true)
    (Variables|Movement|SetRotation 0.0)))

(event Custom|Reload_Event
  (bind _primarywactorref (Variables|References|GetPrimaryWActorRef))
  (bind _primarywactorref_2 (Variables|References|GetPrimaryWActorRef))
  (bind _abpinstance (Variables|References|GetABPInstance))
  ;[1 1 1] Reloading
  (if (not (Variables|UtilytyBooleans|Getb_AimingDownSights))
    _
    (else
      (CallFunction|AimEvent)))
  (if (and (not (Variables|/Game/Characters/Player/ABP_PlayerCharacter.ABP_PlayerCharacter_C|Getb_IsReloading _abpinstance)) (> (Variables|/Script/TamSkadLecaTracery.GunParentV2|GetCarryOnAmmo _primarywactorref) 0))
    (Default|StopFireEvent _primarywactorref)
    ;;[1 1 1] to stop firing while reloading
    (Variables|/Game/Guns/BP_Guns/BP_GunBase.BP_GunBase_C|Setb_CanFIre _primarywactorref false)
    (Audio|PlaySoundatLocation "/Game/Guns/Sound/reload.reload" (Transformation|GetWorldLocation (Variables|/Script/Engine.Actor|GetRootComponent _primarywactorref)) "0, 0, 0" 0.3 0.5 0.0 0 0 0)
    (Variables|/Game/Characters/Player/ABP_PlayerCharacter.ABP_PlayerCharacter_C|Setb_IsReloading _abpinstance true)
    (Class|GunParentV2|Reload _primarywactorref_2)
    ;;[1 1 1] anim time delay
    (Utilities|FlowControl|Delay (Class|GunParentV2|GetReloadTime _primarywactorref_2))
    (Variables|/Game/Characters/Player/ABP_PlayerCharacter.ABP_PlayerCharacter_C|Setb_IsReloading _abpinstance false)
    ;;[1 1 1] to enable firing
    (Variables|/Game/Guns/BP_Guns/BP_GunBase.BP_GunBase_C|Setb_CanFIre (Variables|References|GetPrimaryWActorRef) true)
    ;;[1 1 1] Because <Reasons>
    (Utilities|FlowControl|Delay 0.1)
    (Weapon|UpdateAmmo)))

(event Custom|Aim_Event
  ;[1 1 1] Aim down sights
  (if (not (Variables|UtilytyBooleans|Getb_IsTps))
    (bind _returnvalue (Utilities|Time|SetTimerbyFunctionName 0 "ADS" (Utilities|Time|GetWorldDeltaSeconds) true))
    (if (not (Variables|UtilytyBooleans|Getb_AimingDownSights))
      (Variables|/Script/Engine.CharacterMovementComponent|SetMaxWalkSpeed (Variables|Character|GetCharacterMovement) (Variables|Movement|GetWalkSpeed))
      (Variables|UtilytyBooleans|Setb_AimingDownSights true)
      (else
        ;;[1 1 1] If walk key isnt pressed, move max speed to normal value
        (Variables|UtilytyBooleans|Setb_AimingDownSights false)
        (if (not (Variables|UtilytyBooleans|Getb_IsWalking))
          (Variables|/Script/Engine.CharacterMovementComponent|SetMaxWalkSpeed (Variables|Character|GetCharacterMovement) (Variables|Movement|GetJogSpeed)))
        ;;[1 1 1] snap to socket
        (Transformation|AttachComponentToComponent (Variables|Default|GetFPCamera) (Variables|Default|GetFPCameraSlot) "None" "SnapToTarget" "SnapToTarget" "SnapToTarget" true)
        (Utilities|FlowControl|Delay 0.3)
        (Utilities|Time|ClearandInvalidateTimerbyHandle _returnvalue)))))

(event Input|ActionEvents|InputActionReload
  (params (Key :type Key%20Structure :default "None"))
  (:Pressed
    (CallFunction|ReloadEvent)))

(event Input|ActionEvents|InputActionAim
  (params (Key :type Key%20Structure :default "None"))
  ;[1 1 1] Aim down sights
  (:Pressed
    (CallFunction|AimEvent)))

(event Input|ActionEvents|InputActionFire
  (params (Key :type Key%20Structure :default "None"))
  (bind _primarywactorref (Variables|References|GetPrimaryWActorRef))
  ;[1 1 1] Fire event, calls Fire event on Weapon BP
  (:Pressed
    (if (not (Variables|/Game/Characters/Player/ABP_PlayerCharacter.ABP_PlayerCharacter_C|Getb_IsReloading (Variables|References|GetABPInstance)))
      (Default|FireEvent _primarywactorref)
      ;[1 1 1] Reload while mag is empty
      (if (not (Class|GunParentV2|IsReadytoFire _primarywactorref))
        (if (> (Variables|/Script/TamSkadLecaTracery.GunParentV2|GetCarryOnAmmo _primarywactorref) 0)
          (CallFunction|ReloadEvent)))))
  (:Released
    (Variables|/Game/Characters/Player/ABP_PlayerCharacter.ABP_PlayerCharacter_C|Setb_isFiring (Variables|References|GetABPInstance) false)
    (Default|StopFireEvent (Variables|References|GetPrimaryWActorRef))))

(event EventTakeDMG
  (params (DMGToTake :type Integer) (DmgForce :type Vector :default "0, 0, 0") (ForceLocation :type Vector :default "0, 0, 0") (PlayerControllerID :type Integer) (ControllerRef :type Actor%20Object%20Reference))
  (bind _returnvalue (Components|GetOwner))
  (bind _hud (Variables|References|GetHud))
  (bind _abpinstance (Variables|References|GetABPInstance))
  (bind _mesh (Variables|Character|GetMesh))
  ;[1 1 1] when taking damage
  (if (Variables|UtilytyBooleans|Getb_IsAlive)
    (bind _returnvalue_2 (Class|DefaultCH|GetHp))
    (Class|DefaultCH|SetHp (- _returnvalue_2 DMGToTake))
    ;[1 1 1] Prevents accesed none when not possesed by player
    (if (!= _hud 0)
      (Variables|/Game/Characters/Widgets/W_Hud.W_Hud_C|SetHP _hud (Math|Integer|Clamp(Integer) (- _returnvalue_2 DMGToTake) 0 9999)))
    ;[1 1 1] when players dying
    (bind _returnvalue_3 (Class|DefaultCH|GetHp))
    (if (< _returnvalue_3 1)
      (if (Utilities|DoesObjectImplementInterface ControllerRef "/Game/BPInterfaces/BPI_Afterlife.BPI_Afterlife_C")
        ;;[1 1 1] add kill to damage dealer
        (Class|BPIAfterlife|AddKill(Message) ControllerRef))
      (Variables|UtilytyBooleans|Setb_IsAlive false)
      (Variables|/Game/Characters/Player/ABP_PlayerCharacter.ABP_PlayerCharacter_C|Setb_IsAlive (Variables|References|GetABPInstance) false)
      ;;[1 1 1] CH feeling cold
      (Input|DisableInput 0)
      (if (not (Variables|UtilytyBooleans|Getb_IsTps))
        (CallFunction|SwitchCamEvent))
      (if (not (or (or (> DMGToTake 50) (> (Variables|/Game/Characters/Player/ABP_PlayerCharacter.ABP_PlayerCharacter_C|GetSpeed _abpinstance) 1e+01)) (Variables|/Game/Characters/Player/ABP_PlayerCharacter.ABP_PlayerCharacter_C|GetJumping _abpinstance)))
        ;;[1 1 1] wait for animation to play
        (Utilities|FlowControl|Delay 2.0)
        ;;[1 1 1] Ragdoll version
        (Collision|SetCollisionEnabled (Variables|Default|GetCapsuleComponent) "NoCollision")
        (Collision|SetCollisionEnabled (Variables|Character|GetMesh) "PhysicsOnly")
        (Physics|SetSimulatePhysics (Variables|Character|GetMesh) true)
        (else
          ;;[1 1 1] just wait for switch cam
          (Utilities|FlowControl|Delay 0.1)
          ;[1 1 1] Add force for ragdoll
          (Collision|SetCollisionEnabled (Variables|Default|GetCapsuleComponent) "NoCollision")
          (Collision|SetCollisionEnabled (Variables|Character|GetMesh) "PhysicsOnly")
          (Physics|SetSimulatePhysics _mesh true)
          (Class|PrimitiveComponent|WakeRigidBody _mesh "None")
          (Class|PrimitiveComponent|AddForceatLocation _mesh (* DmgForce (Math|Conversions|ToInteger(Byte) (Class|KismetMathLibrary|RandomInteger64inRange 75 150))) ForceLocation (.ReturnValue (Class|SkinnedMeshComponent|FindClosestBoneK2 (Variables|Character|GetMesh) ForceLocation 0.0)))))
      (if (Utilities|DoesObjectImplementInterface _returnvalue "/Game/BPInterfaces/BPI_Afterlife.BPI_Afterlife_C")
        ;[1 1 1] Soul leaving the body
        (Class|BPIAfterlife|DeathEvent(Message) _returnvalue)))))

(fn ConstructionScript
  ;[1 1 1] hitboxes visibility in viewport
  (Rendering|SetVisibility (Variables|HitBoxes|GetULegL) false false)
  ;[1 1 1] set default values from data table
  (Utilities|SetupCHValuesfromDataTable))

(fn GetABPReference
  (bind _asabp_player_character (Utilities|Casting|CastToABP_PlayerCharacter (Components|SkeletalMesh|GetAnimInstance (Variables|Character|GetMesh)))
    (:then
      (Variables|References|SetABPInstance _asabp_player_character))
    (:CastFailed
      (Development|PrintString "Cast to ABPEU$ASSP HERO failed"))))

(fn SetSpeedandDirection
  (bind _abpinstance (Variables|References|GetABPInstance))
  (Variables|/Game/Characters/Player/ABP_PlayerCharacter.ABP_PlayerCharacter_C|SetDirectionV2 _abpinstance (Class|DefaultCH|CalculateMovementDirection))
  (Variables|/Game/Characters/Player/ABP_PlayerCharacter.ABP_PlayerCharacter_C|SetSpeed _abpinstance (Math|Vector|VectorLength (Transformation|GetVelocity))))

(fn ADS
  (bind _fpcamera (Variables|Default|GetFPCamera))
  (bind _fpcamera_2 (Variables|Default|GetFPCamera))
  (if (Variables|UtilytyBooleans|Getb_AimingDownSights)
    ;[1 1 1] Move to socket on weapon to  attaching
    (Transformation|SetWorldLocation (Variables|Default|GetFPCamera) (Math|Interpolation|VInterpTo (Transformation|GetWorldLocation (Variables|Default|GetFPCamera)) (Transformation|GetWorldLocation (Components|GetChildComponent (Variables|/Script/Engine.Actor|GetRootComponent (Variables|/Script/Engine.ChildActorComponent|GetChildActor (Variables|Default|GetPrimaryWeapon))) 0)) (Utilities|Time|GetWorldDeltaSeconds) (Variables|Movement|GetAimingTime)) false false)
    ;[1 1 1] Change fov over time for nice effect
    (Camera|SetFieldOfView _fpcamera (Math|Interpolation|FInterpTo (Variables|/Script/Engine.CameraComponent|GetFieldOfView _fpcamera) (Variables|Default|GetAimFov) (Utilities|Time|GetWorldDeltaSeconds) (Variables|Movement|GetAimingTime)))
    (else
      ;[1 1 1] move to socket on head for attaching
      (Transformation|SetWorldLocation (Variables|Default|GetFPCamera) (Math|Interpolation|VInterpTo (Transformation|GetWorldLocation (Variables|Default|GetFPCamera)) (Transformation|GetWorldLocation (Variables|Default|GetFPCameraSlot)) (Utilities|Time|GetWorldDeltaSeconds) (Variables|Movement|GetAimingTime)) false false)
      (Camera|SetFieldOfView _fpcamera_2 (Math|Interpolation|FInterpTo (Variables|/Script/Engine.CameraComponent|GetFieldOfView _fpcamera_2) (Variables|Default|GetFov) (Utilities|Time|GetWorldDeltaSeconds) (Variables|Movement|GetAimingTime))))))

(fn SetPrimaryWActorRef
  (bind _asbp_gun_base (Utilities|Casting|CastToBP_GunBase (Variables|/Script/Engine.ChildActorComponent|GetChildActor (Variables|Default|GetPrimaryWeapon))))
  (Variables|References|SetPrimaryWActorRef _asbp_gun_base))

(fn UpdateAmmo
  (if (!= (Variables|References|GetHud) 0)
    (Variables|/Game/Characters/Widgets/W_Hud.W_Hud_C|SetAmmo (Variables|References|GetHud) (Class|GunParentV2|GetAmmoLeft (Variables|References|GetPrimaryWActorRef)))))

(fn UpdateFireStatus
  (bind _returnvalue (Utilities|Time|GetWorldDeltaSeconds))
  (bind _primarywactorref (Variables|References|GetPrimaryWActorRef))
  (bind _b_canfire (Variables|/Game/Guns/BP_Guns/BP_GunBase.BP_GunBase_C|Getb_CanFIre _primarywactorref))
  ;[1 1 1] UPdates Ammo then firing status for anim
  (Weapon|UpdateAmmo)
  (if _b_canfire
    (bind _output_get (Variables|/Game/Characters/Player/ABP_PlayerCharacter.ABP_PlayerCharacter_C|Setb_isFiring (Variables|References|GetABPInstance) (and _b_canfire (Class|GunParentV2|IsReadytoFire _primarywactorref))))
    (if _output_get
      (Pawn|Input|AddControllerPitchInput (* _returnvalue -7.0))
      (Pawn|Input|AddControllerYawInput (* _returnvalue (* (Math|Integer|Clamp(Integer) (Variables|Default|GetXtickss) -1 1) 2.0)))
      ;[1 1 1] set recoil X TODO move this sphagetti to cpp
      (if (== (Variables|Default|GetXtickss) 0)
        (Variables|Default|SetXtickss (- (Math|Random|RandomInteger 59) 30))
        (elif (> (Variables|Default|GetXtickss) 0)
          (Variables|Default|SetXtickss (- (Variables|Default|GetXtickss) 1))
          (else
            (Variables|Default|SetXtickss (+ (Variables|Default|GetXtickss) 1))))))
    (else
      (Variables|/Game/Characters/Player/ABP_PlayerCharacter.ABP_PlayerCharacter_C|Setb_isFiring (Variables|References|GetABPInstance) false))))

(fn ChangeCam
  (params (TargetDestination :type Vector) (InterpSpeed :type Float%20%28single-precision%29))
  ;[1 1 1] Move to socket on weapon to  attaching
  (Transformation|SetWorldLocation (Variables|Default|GetFPCamera) (Math|Interpolation|VInterpTo (Transformation|GetWorldLocation (Variables|Default|GetFPCamera)) TargetDestination (Utilities|Time|GetWorldDeltaSeconds) InterpSpeed) false false))

(fn MoveOutOftheWall
  (bind _returnvalue (Pawn|GetControlRotation :!class /Script/Engine.Pawn))
  (bind _returnvalue_2 (Pawn|GetControlRotation :!class /Script/Engine.Pawn))
  (bind _returnvalue_3 (Math|Rotator|MakeRotator 0.0 0.0 (.yaw _returnvalue_2)))
  (bind _returnvalue_4 (Math|Vector|GetForwardVector _returnvalue_3))
  (if (not (and (> (.pitch _returnvalue) 5e+01) (< (.pitch _returnvalue) 91.0)))
    (Pawn|Input|AddMovementInput _returnvalue_4 -1e+01 false)
    (else
      (Pawn|Input|AddMovementInput _returnvalue_4 1e+01 false))))

(fn SetupGunVariablesinABP
  (bind _abpinstance (Variables|References|GetABPInstance))
  (Variables|/Game/Characters/Player/ABP_PlayerCharacter.ABP_PlayerCharacter_C|SetFiringAnimationSpeed _abpinstance (/ (Class|GunParentV2|GetShotsPerMinute (Variables|References|GetPrimaryWActorRef)) 6e+02))
  (bind _returnvalue (Utilities|GetDataTableRow "/Game/Guns/DataTables/Table_GunValues.Table_GunValues" (Utilities|String|StringToName (Utilities|GetClassDisplayName (Utilities|GetClass (Variables|References|GetPrimaryWActorRef)))))
    (:then
      (Variables|/Game/Characters/Player/ABP_PlayerCharacter.ABP_PlayerCharacter_C|SetTimeToFullRecoil _abpinstance (.timetofullrecoil _returnvalue))
      (Variables|/Game/Characters/Player/ABP_PlayerCharacter.ABP_PlayerCharacter_C|SetTimeOutFromFullRecoil _abpinstance (.timeoutfromfullrecoil _returnvalue)))
    (:RowNotFound
      (Development|PrintString "cant setup CH weapon variabless"))))