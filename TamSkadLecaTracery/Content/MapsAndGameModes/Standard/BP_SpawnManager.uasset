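; BP_SpawnManager is the Standard mode actor that manages spawn points and spawns player characters.
; On BeginPlay it registers itself on GS_Standard, with an immediate, delay-free retry if the cast result is invalid; a failed cast simply stops.
; Show and hide events toggle the lights on every spawn point.
; RequestRespawnNewPawn spawns and returns a BP_PlayerCH at a spawn point's location with a primary gun ID, without possessing it.
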(event Custom|Retry
  (bind _asgs_standard (Utilities|Casting|CastToGS_Standard (Game|GetGameState)))
  (Utilities|IsValid _asgs_standard
    (:Is%20Valid
      (Variables|/Game/MapsAndGameModes/Standard/GS_Standard.GS_Standard_C|SetSpawnManagerReference _asgs_standard self))
    (:Is%20Not%20Valid
      (CallFunction|Retry)
      (Development|PrintString "SpawnManagerRetry"))))

(event Custom|EVENT_ShowSpawns
  ;[1 1 1] turn on light on spawns
  (for _array_element (Variables|Default|GetSpawnPoints)
    (Default|EVENTShowSpawn _array_element)))

(event Custom|EVENT_HideSpawns
  ;[1 1 1] turn off light on spawns
  (for _array_element (Variables|Default|GetSpawnPoints)
    (Default|EVENTHideSpawn _array_element)))

(event EventBeginPlay
  (bind _asgs_standard (Utilities|Casting|CastToGS_Standard (Game|GetGameState)))
  (Utilities|IsValid _asgs_standard
    (:Is%20Valid
      (Variables|/Game/MapsAndGameModes/Standard/GS_Standard.GS_Standard_C|SetSpawnManagerReference _asgs_standard self))
    (:Is%20Not%20Valid
      (CallFunction|Retry)
      (Development|PrintString "SpawnManagerRetry"))))

(event Collision|EventActorBeginOverlap
  (params (OtherActor :type Actor%20Object%20Reference)))

(event EventTick
  (params (DeltaSeconds :type Float%20%28single-precision%29)))

(fn ConstructionScript)

(fn RequestRespawnNewPawn
  (params (SpawnPoint :type BP%20Spawn%20Point%20Object%20Reference) (PrimaryGunID :type E_GunID%20Enum :default "AR"))
  (bind _returnvalue (Game|SpawnActorfromClass "/Game/Characters/Player/BP_PlayerCH.BP_PlayerCH_C" (Math|Transform|MakeTransform (Transformation|GetActorLocation SpawnPoint) "0, 0, 0" "1,1,1") "Undefined" 0 PrimaryGunID 0))
  (return _returnvalue))