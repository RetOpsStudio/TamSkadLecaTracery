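; BP_AR is a gun Blueprint, still at a placeholder stage of its firing logic.
; The Fire input press and a custom fire event both lead to a debug "Hello" print.
; A node that would spawn BP_Bullet at the skeletal mesh's Bullet socket is present but unconnected, so no projectile spawns.
; Tick and the construction script only call their parents.
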(event Custom|Fire_Event_0
  (Development|PrintString "Hello"))

(event EventBeginPlay
  (|CallParentFunction) ; This node is disabled and will not be called.\nDrag off pins to build functionality.
)

(event Collision|EventActorBeginOverlap
  (params (OtherActor :type Actor%20Object%20Reference))
  (|CallParentFunction OtherActor) ; This node is disabled and will not be called.\nDrag off pins to build functionality.
)

(event EventTick
  (params (DeltaSeconds :type Float%20%28single-precision%29))
  (|CallParentFunction DeltaSeconds))

(event Input|ActionEvents|InputActionFire
  (params (Key :type Key%20Structure))
  (:Pressed
    (Development|PrintString "Hello")))

(fn ConstructionScript
  (|CallParentFunction))