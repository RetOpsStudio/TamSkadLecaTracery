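; Player controller that sets up the HUD, opens the in-game menu and handles a work-in-progress respawn.
; On begin play it creates the HUD, caches the character and its primary gun, and pushes current HP to the HUD.
; The death event clears widgets, waits briefly, spawns and possesses a new character at the first PlayerStart, then reruns setup.
; It also counts kills and deaths, printing each update.
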(event Custom|Death_Event
  ;[1 1 1] Respawn (Work in Progress)
  (Viewport|RemoveAllWidgets)
  (Pawn|UnPossess)
  (bind _outactors (Actor|GetAllActorsOfClass "/Script/Engine.PlayerStart"))
  (Utilities|FlowControl|Delay 1.0)
  (bind _returnvalue (Game|SpawnActorfromClass "/Game/CH/CH_PlayerCharacter.CH_PlayerCharacter_C" (Transformation|GetActorTransform (Utilities|Array|Get(acopy) _outactors)) "AlwaysSpawn" self 0))
  (Pawn|Possess _returnvalue)
  (CallFunction|SetupWidgetsandReferences))

(event EventBeginPlay
  ;[1 1 1] Setup Pawn References
  (CallFunction|SetupWidgetsandReferences))

(event Input|ActionEvents|InputActionMenu
  (params (Key :type Key%20Structure :default "None"))
  ;[1 1 1] Open ingame Menu
  (:Pressed
    (bind _returnvalue (UserInterface|CreateWidget "/Game/CH/Widgets/W_GameMenu.W_GameMenu_C" self))
    (UserInterface|Viewport|AddtoViewport _returnvalue 0)))

(fn ConstructionScript)

(fn AddKill
  (bind _result (Math|Integer|IncrementInt (Variables|Default|GetKills))
    (:%20%20
      (Variables|Default|SetKills _result)
      (Development|PrintString (Utilities|String|ToString(Integer) (Variables|Default|GetKills))))))

(fn AddDeath
  (bind _result (Math|Integer|IncrementInt (Variables|Default|GetDeaths))
    (:%20%20
      (Variables|Default|SetDeaths _result)
      (Development|PrintString (Utilities|String|ToString(Integer) (Variables|Default|GetDeaths))))))

(fn SetupWidgetsandReferences
  (bind _returnvalue (UserInterface|CreateWidget "/Game/CH/Widgets/W_Hud.W_Hud_C"))
  (Variables|Default|SetHudRef _returnvalue)
  (bind _asch_player_character (Utilities|Casting|CastToCH_PlayerCharacter (Pawn|GetControlledPawn)))
  (bind _output_get (Variables|Default|SetCH _asch_player_character))
  (bind _asbp_gun_base (Utilities|Casting|CastToBP_GunBase (Variables|/Script/Engine.ChildActorComponent|GetChildActor (Variables|/Game/CH/CH_PlayerCharacter.CH_PlayerCharacter_C|GetPrimaryWeapon _output_get))))
  (Variables|Default|SetGunRef _asbp_gun_base)
  (UserInterface|Viewport|AddtoViewport _returnvalue 0)
  (Variables|/Game/CH/CH_PlayerCharacter.CH_PlayerCharacter_C|SetHud (Variables|Default|GetCH) (Variables|Default|GetHudRef))
  (bind _returnvalue_2 (Class|DefaultCH|GetHp (Variables|Default|GetCH)))
  (Variables|/Game/CH/Widgets/W_Hud.W_Hud_C|SetHP (Variables|Default|GetHudRef) _returnvalue_2))