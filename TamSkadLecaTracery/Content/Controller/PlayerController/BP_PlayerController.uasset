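; Player controller that owns the HUD, the in-game menu, per-player kill and death counts, and the player's team.
; On BeginPlay it creates the HUD widget and links it to the controlled BP_PlayerCH, seeding its HP.
; DeathEvent, a work-in-progress respawn, counts the death, removes the HUD, spawns and possesses a new character at the first PlayerStart after a delay, then decreases team tickets in GM_StandardMode.
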(event EventBeginPlay
  ;[1 1 1] Setup Pawn References
  (CallFunction|SetupWidgetsandReferences))

(event EventDeathEvent
  ;[1 1 1] Respawn (Work in Progress)
  ;;[1 1 1] remove HUD from Viewport
  (CallFunction|IncreaseDeaths)
  (Widget|RemovefromParent (Variables|Default|GetHudRef))
  (Pawn|UnPossess)
  ;;[1 1 1] Spawn and posess new pawn
  (bind _outactors (Actor|GetAllActorsOfClass "/Script/Engine.PlayerStart"))
  (Utilities|FlowControl|Delay 1.0)
  (bind _returnvalue (Game|SpawnActorfromClass "/Game/Characters/Player/BP_PlayerCH.BP_PlayerCH_C" (Transformation|GetActorTransform (Utilities|Array|Get(acopy) _outactors)) "AlwaysSpawn" self 0))
  (Pawn|Possess _returnvalue)
  (CallFunction|SetupWidgetsandReferences)
  (bind _asgm_standard_mode (Utilities|Casting|CastToGM_StandardMode (Game|GetGameMode)))
  (Default|DecreaseTickets _asgm_standard_mode 1 (Variables|Default|GetMyTeam_0)))

(event EventPossess
  (params (PossessedPawn :type Pawn%20Object%20Reference))
  ;[1 1 1] Setup Pawn References
)

(event EventAddKill
  (CallFunction|IncreaseKills))

(event EventAddDeath
  (CallFunction|IncreaseDeaths))

(event Input|ActionEvents|InputActionMenu
  (params (Key :type Key%20Structure :default "None"))
  ;[1 1 1] Open ingame Menu
  (:Pressed
    (bind _returnvalue (UserInterface|CreateWidget "/Game/Characters/Widgets/W_GameMenu.W_GameMenu_C" self))
    (UserInterface|Viewport|AddtoViewport _returnvalue 0)))

(fn ConstructionScript)

(fn IncreaseKills
  (bind _result (Math|Integer|IncrementInt (Variables|Default|GetKills))
    (:%20%20
      (Variables|Default|SetKills _result)
      (Development|PrintString (Utilities|String|ToString(Integer) (Variables|Default|GetKills)))
      (Development|PrintString (Variables|Default|GetName)))))

(fn IncreaseDeaths
  (bind _result (Math|Integer|IncrementInt (Variables|Default|GetDeaths))
    (:%20%20
      (Variables|Default|SetDeaths _result)
      (Development|PrintString (Utilities|String|ToString(Integer) (Variables|Default|GetDeaths)))
      (Development|PrintString (Class|KismetSystemLibrary|GetGameName)))))

(fn SetupWidgetsandReferences
  (bind _returnvalue (UserInterface|CreateWidget "/Game/Characters/Widgets/W_Hud.W_Hud_C"))
  (Variables|Default|SetHudRef _returnvalue)
  (bind _asbp_player_ch (Utilities|Casting|CastToBP_PlayerCH (Pawn|GetControlledPawn)))
  (Variables|Default|SetCH _asbp_player_ch)
  (UserInterface|Viewport|AddtoViewport _returnvalue 0)
  (Variables|/Game/Characters/Player/BP_PlayerCH.BP_PlayerCH_C|SetHud (Variables|Default|GetCH) (Variables|Default|GetHudRef))
  (bind _returnvalue_2 (Class|DefaultCH|GetHp (Variables|Default|GetCH)))
  (Variables|/Game/Characters/Widgets/W_Hud.W_Hud_C|SetHP (Variables|Default|GetHudRef) _returnvalue_2))

(fn GetTeam
  (return (Variables|Default|GetMyTeam_0)))