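; Selectable spawn point actor with a widget and spotlight, which can be shown or hidden in game.
; On BeginPlay it links itself to its widget, then after a short delay registers with the GS_Standard game state's spawn manager.
; A button press on an unselected point turns all registered spotlights red, deselects the previous point, then selects itself with an explosion, text animation and sequence.
; The green highlight code is disconnected.
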(event Custom|EVENT_ShowSpawn
  (Rendering|SetActorHiddenInGame self false))

(event Custom|EVENT_HideSpawn
  (Rendering|SetActorHiddenInGame self true))

(event Custom|EVENT_SpawnButtonPressed
  (bind _widgetobjectreference (Variables|Default|GetWidgetObjectReference))
  ;[1 1 1] Change selected spawn
  (if (not (Variables|Default|Getb_IsSelected))
    (bind _asgs_standard (Utilities|Casting|CastToGS_Standard (Game|GetGameState)))
    (for _array_element (Variables|/Game/GameModes/Standard/BP_SpawnManager.BP_SpawnManager_C|GetSpawnPoints (Variables|/Game/GameModes/Standard/GS_Standard.GS_Standard_C|GetSpawnManagerReference _asgs_standard))
      (Rendering|Components|Light|SetLightColor (Variables|BP_SpawnPoint_C|GetSpotLight _array_element) "(R=0.375000,G=0.000000,B=0.007161,A=1.000000)" true)
      (if (Variables|BP_SpawnPoint_C|Getb_IsSelected _array_element)
        (Class|UserWidget|PlayAnimationReverse (Variables|BP_SpawnPoint_C|GetWidgetObjectReference _array_element) (Variables|/Game/Characters/Widgets/W_Spawn.W_Spawn_C|GetShowText (Variables|BP_SpawnPoint_C|GetWidgetObjectReference _array_element)) 1.0 false)
        (Variables|BP_SpawnPoint_C|Setb_IsSelected _array_element false)))
    (Variables|Default|Setb_IsSelected true)
    (Effects|SpawnEmitteratLocation "/Game/StarterContent/Particles/P_Explosion.P_Explosion" (Transformation|GetWorldLocation (Variables|Default|GetDefaultSceneRoot)))
    (Class|UserWidget|PlayAnimationForward _widgetobjectreference (Variables|/Game/Characters/Widgets/W_Spawn.W_Spawn_C|GetShowText _widgetobjectreference) 1.0 false)
    (Sequencer|Player|Play (Variables|/Script/ActorSequence.ActorSequenceComponent|GetSequencePlayer (Variables|Default|GetActorSequence)) :!class /Script/MovieScene.MovieSceneSequencePlayer)))

(event EventBeginPlay
  ;[1 1 1] set owner in widget
  (bind _output_get (Variables|Default|SetWidgetObjectReference (.AsW%20Spawn (Utilities|Casting|CastToW_Spawn (UserInterface|GetUserWidgetObject (Variables|Default|GetWidget))))))
  (Variables|/Game/Characters/Widgets/W_Spawn.W_Spawn_C|SetOwner _output_get self)
  ;[1 1 1] add self to list of avalible spawn points in spawn manager
  (bind _asgs_standard (Utilities|Casting|CastToGS_Standard (Game|GetGameState)))
  (Utilities|FlowControl|Delay 1.0)
  (Utilities|IsValid (Variables|/Game/GameModes/Standard/GS_Standard.GS_Standard_C|GetSpawnManagerReference _asgs_standard)
    (:Is%20Valid
      (Utilities|Array|Add (Variables|/Game/GameModes/Standard/BP_SpawnManager.BP_SpawnManager_C|GetSpawnPoints (Variables|/Game/GameModes/Standard/GS_Standard.GS_Standard_C|GetSpawnManagerReference _asgs_standard)) self))
    (:Is%20Not%20Valid
      (Development|PrintString "SpawnPoint:Cant add to Spawn manager reference to self"))))

(event Collision|EventActorBeginOverlap
  (params (OtherActor :type Actor%20Object%20Reference)))

(event EventTick
  (params (DeltaSeconds :type Float%20%28single-precision%29)))

(fn ConstructionScript)