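; Default player character Blueprint handling look, movement, walk, jump, crouch and a toggle of the first-person camera.
; On BeginPlay it caches the hero TPP AnimBlueprint instance for input events to update directly.
; Movement follows control rotation and feeds speed and direction to animation, while jump and crouch flip animation flags.
; Look input drives controller yaw and pitch, with pitch input also re-aligning the third-person spring arm.
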(event EventBeginPlay
  (CallFunction|GetABPReference)
  (Class|DefaultCH|SetupVariables (Variables|Default|GetABPInstance)))

(event Collision|EventActorBeginOverlap
  (params (OtherActor :type Actor%20Object%20Reference)))

(event EventTick
  (params (DeltaSeconds :type Float%20%28single-precision%29)))

(event Input|ActionEvents|InputActionJump
  (params (Key :type Key%20Structure :default "None"))
  (bind _abpinstance (Variables|Default|GetABPInstance))
  ;[1 1 1] Movement
  ;;[1 1 1] Jumping
  (:Pressed
    (Variables|/Game/CH/UE4ASP_HeroTPP_AnimBlueprint.UE4ASP_HeroTPP_AnimBlueprint_C|SetEnable%20Jump _abpinstance (not (Variables|/Game/CH/UE4ASP_HeroTPP_AnimBlueprint.UE4ASP_HeroTPP_AnimBlueprint_C|GetEnable%20Jump _abpinstance)))
    (Character|Jump)
    (Utilities|FlowControl|Delay 0.2)
    (Variables|/Game/CH/UE4ASP_HeroTPP_AnimBlueprint.UE4ASP_HeroTPP_AnimBlueprint_C|SetEnable%20Jump _abpinstance (not (Variables|/Game/CH/UE4ASP_HeroTPP_AnimBlueprint.UE4ASP_HeroTPP_AnimBlueprint_C|GetEnable%20Jump _abpinstance)))))

(event Input|ActionEvents|InputActionCrouch
  (params (Key :type Key%20Structure :default "None"))
  (bind _abpinstance (Variables|Default|GetABPInstance))
  ;[1 1 1] Movement
  ;;[1 1 1] Crouching
  (:Pressed
    (Variables|/Game/CH/UE4ASP_HeroTPP_AnimBlueprint.UE4ASP_HeroTPP_AnimBlueprint_C|SetCrouching _abpinstance (not (Variables|/Game/CH/UE4ASP_HeroTPP_AnimBlueprint.UE4ASP_HeroTPP_AnimBlueprint_C|GetCrouching _abpinstance)))
    (Utilities|FlowControl|FlipFlop
      (:A
        (Character|Crouch))
      (:B
        (Character|UnCrouch)))))

(event Input|ActionEvents|InputActionCameraSwitch
  (params (Key :type Key%20Structure :default "None"))
  ;[1 1 1] Switch Camera
  (:Pressed
    (Components|Activation|ToggleActive (Variables|Default|GetFPCamera))))

(event Input|ActionEvents|InputActionwalk
  (params (Key :type Key%20Structure :default "None"))
  (bind _charactermovement (Variables|Character|GetCharacterMovement))
  ;[1 1 1] Movement
  ;;[1 1 1] Walking
  (:Pressed
    (Variables|/Script/Engine.CharacterMovementComponent|SetMaxWalkSpeed _charactermovement 2e+02))
  (:Released
    (Variables|/Script/Engine.CharacterMovementComponent|SetMaxWalkSpeed _charactermovement 4e+02)))

(event Input|AxisEvents|InputAxisMovCamY
  (params (AxisValue :type Float%20%28single-precision%29))
  (bind _returnvalue (Pawn|GetControlRotation :!class /Script/Engine.Pawn))
  ;[1 1 1] RotationXY
  (Variables|/Game/CH/UE4ASP_HeroTPP_AnimBlueprint.UE4ASP_HeroTPP_AnimBlueprint_C|SetRotationY (Variables|Default|GetABPInstance) 0.0) ; FOR ABP
  (Pawn|Input|AddControllerPitchInput (* -1 AxisValue))
  (Variables|Default|SetRotation 0.0)
  ;[1 1 1] Switch Camera
  ;;[1 1 1] 3PS SpringArm rotation
  (Transformation|SetRelativeRotation (Variables|Default|GetSpringArm) (Math|Rotator|MakeRotator (.roll _returnvalue) (.pitch _returnvalue) (- (.yaw _returnvalue) 9e+01)) false false))

(event Input|AxisEvents|InputAxisMovForwardBackward
  (params (AxisValue :type Float%20%28single-precision%29))
  ;[1 1 1] Movement
  ;;[1 1 1] WSAD
  (Pawn|Input|AddMovementInput (Math|Vector|GetForwardVector (Pawn|GetControlRotation :!class /Script/Engine.Pawn)) (Math|Float|Sign(Float) AxisValue) false)
  ;;[1 1 1] Calc and sed direction in ABP
  (CallFunction|SetSpeedandDirection))

(event Input|AxisEvents|InputAxisMovLeftRight
  (params (AxisValue :type Float%20%28single-precision%29))
  ;[1 1 1] Movement
  ;;[1 1 1] WSAD
  (Pawn|Input|AddMovementInput (Math|Vector|GetRightVector (Pawn|GetControlRotation :!class /Script/Engine.Pawn)) AxisValue false)
  ;;[1 1 1] Calc and sed direction in ABP
  (CallFunction|SetSpeedandDirection))

(event Input|AxisEvents|InputAxisMovCamX
  (params (AxisValue :type Float%20%28single-precision%29))
  ;[1 1 1] RotationXY
  (Variables|Default|SetRotation 0.0)
  ;[1 1 1] move spine
  (Default|ItsMeDio (Variables|Default|GetABPInstance))
  (Pawn|Input|AddControllerYawInput AxisValue)
  (if true
    (Variables|/Game/CH/UE4ASP_HeroTPP_AnimBlueprint.UE4ASP_HeroTPP_AnimBlueprint_C|SetDiff (Variables|Default|GetABPInstance) 0.0))
  (Development|PrintString "Hello"))

(fn ConstructionScript)

(fn GetABPReference
  (bind _asue4asp_hero_tpp_anim_blueprint (Utilities|Casting|CastToUE4ASP_HeroTPP_AnimBlueprint (Components|SkeletalMesh|GetAnimInstance (Variables|Character|GetMesh)))
    (:then
      (Variables|Default|SetABPInstance _asue4asp_hero_tpp_anim_blueprint))
    (:CastFailed
      (Development|PrintString "Cast to ABPEU$ASSP HERO failed"))))

(fn SetSpeedandDirection
  (bind _abpinstance (Variables|Default|GetABPInstance))
  (Variables|/Game/CH/UE4ASP_HeroTPP_AnimBlueprint.UE4ASP_HeroTPP_AnimBlueprint_C|SetDirectionV2 _abpinstance (Class|DefaultCH|CalculateMovementDirection))
  (Variables|/Game/CH/UE4ASP_HeroTPP_AnimBlueprint.UE4ASP_HeroTPP_AnimBlueprint_C|SetSpeed _abpinstance (Math|Vector|VectorLength (Transformation|GetVelocity))))