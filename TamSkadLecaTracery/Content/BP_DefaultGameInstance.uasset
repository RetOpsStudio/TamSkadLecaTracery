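; BP_DefaultGameInstance is a game instance Blueprint that handles multiplayer session events on top of C++ session functionality.
; When a session search finishes, the C++-invoked event fires the search-complete dispatcher, and a network error destroys the session.
; Init is empty, and a disconnected debug loop that prints each search result's server details and joins it never runs.
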(event EventInit)

(event EventHandleNetworkError
  (params (FailureType :type ENetworkFailure%20Enum :default "NetDriverAlreadyExists") (bIsServer :type Boolean))
  (Class|GameInstanceParent|DestroySession))

(event EventOnSearchSessionsFinishedEvent
  ;[1 1 1] Called in cpp
  (Default|CallSearchGameCompleteDispatcher))