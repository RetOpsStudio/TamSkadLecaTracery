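; Projectile bullet that damages hitboxes, penetrates armor and ricochets off surfaces.
; Hitbox overlaps send damage to BPI_Damageable actors, scaled by hitbox multiplier and remaining speed fraction.
; Armor minus penetration slows the bullet by that percentage, destroying it at or below minimum speed.
; On hits, head-on angle or low speed favors multicast destruction with an emitter; otherwise velocity is randomly damped per axis.
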(event OnComponentBeginOverlap(StaticMesh)
  (params (OverlappedComponent :type Primitive%20Component%20Object%20Reference) (OtherActor :type Actor%20Object%20Reference) (OtherComp :type Primitive%20Component%20Object%20Reference) (OtherBodyIndex :type Integer) (bFromSweep :type Boolean) (SweepResult :type Hit%20Result%20Structure%20%28by%20ref%29))
  (bind _staticmesh (Variables|Default|GetStaticMesh))
  (bind _returnvalue (Transformation|GetComponentVelocity _staticmesh))
  (bind _ashit_box (Utilities|Casting|CastToHitBox OtherComp))
  (bind _returnvalue_2 (Class|BulletParent|GetInitialBulletSpeed))
  (if (Utilities|DoesObjectImplementInterface OtherActor "/Game/BPInterfaces/BPI_Damageable.BPI_Damageable_C")
    (Class|BPIDamageable|TakeDMG(Message) OtherActor (Math|Float|Truncate (* (Class|HitBox|GetDamageMultiplier _ashit_box) (* (Variables|Default|GetBaseDamage) (/ (Math|Vector|VectorLength (Variables|/Script/Engine.MovementComponent|GetVelocity (Variables|Default|GetProjectileMovementComponent))) _returnvalue_2)))) (Variables|/Script/Engine.MovementComponent|GetVelocity (Variables|Default|GetProjectileMovementComponent)) (Transformation|GetWorldLocation _ashit_box) (Variables|Default|GetPlayerControllerID) (Variables|Default|GetPawnControllerRef)))
  ;[1 1 1] if speed is > minimal speed , set new speed/ else destroy bullet
  (if (> (Math|Vector|VectorLength (- _returnvalue (* _returnvalue (/ (Math|Conversions|ToFloat(Integer) (Math|Integer|Clamp(Integer) (- (Class|HitBox|GetArmor _ashit_box) (Variables|Default|GetArmorPene)) 0 100)) 1e+02)))) (Math|Conversions|ToFloat(Integer) (Variables|Default|GetMinimalSpeed)))
    (Variables|/Script/Engine.MovementComponent|SetVelocity (Variables|Default|GetProjectileMovementComponent) (- _returnvalue (* _returnvalue (/ (Math|Conversions|ToFloat(Integer) (Math|Integer|Clamp(Integer) (- (Class|HitBox|GetArmor _ashit_box) (Variables|Default|GetArmorPene)) 0 100)) 1e+02))))
    (else
      (Actor|DestroyActor))))

(event Custom|MULTICAST_DestroyActor
  (params (Location :type Vector%20%28by%20ref%29))
  ;[1 1 1] if cant move along
  (Effects|SpawnEmitteratLocation "/Game/Guns/Particles/P_MuzzleFlash.P_MuzzleFlash" Location)
  (Actor|DestroyActor))

(event Collision|EventActorBeginOverlap
  (params (OtherActor :type Actor%20Object%20Reference)))

(event Collision|EventHit
  (params (MyComp :type Primitive%20Component%20Object%20Reference) (Other :type Actor%20Object%20Reference) (OtherComp :type Primitive%20Component%20Object%20Reference) (bSelfMoved :type Boolean) (HitLocation :type Vector :default "0, 0, 0") (HitNormal :type Vector :default "0, 0, 0") (NormalImpulse :type Vector :default "0, 0, 0") (Hit :type Hit%20Result%20Structure%20%28by%20ref%29))
  (bind _projectilemovementcomponent (Variables|Default|GetProjectileMovementComponent))
  (if (or (< (Math|Random|RandomInteger 100) (Math|Float|Truncate (* (Math|Float|Absolute(Float) (Math|Vector|DotProduct HitNormal (Math|Vector|GetForwardVector (Variables|Default|GetStaticMesh)))) 1e+02))) (< (Math|Vector|VectorLength (Transformation|GetComponentVelocity (Variables|Default|GetStaticMesh))) (Math|Conversions|ToFloat(Integer) (Variables|Default|GetMinimalSpeed))))
    (CallFunction|MULTICASTDestroyActor HitLocation)
    (else
      ;[1 1 1] randomize ricochet
      (Variables|/Script/Engine.MovementComponent|SetVelocity _projectilemovementcomponent (Math|Vector|MakeVector (* (.x (Variables|/Script/Engine.MovementComponent|GetVelocity _projectilemovementcomponent)) (Math|Random|RandomFloatinRange 0.5 1.0)) (* (.y (Variables|/Script/Engine.MovementComponent|GetVelocity _projectilemovementcomponent)) (Math|Random|RandomFloatinRange 0.5 1.0)) (* (.z (Variables|/Script/Engine.MovementComponent|GetVelocity _projectilemovementcomponent)) (Math|Random|RandomFloatinRange 0.5 1.0)))))))

(fn ConstructionScript)