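; Standard Team Deathmatch game mode that scores kills for the Green and Red teams and ends the match.
; AddKillforTeam raises the team's score; once either passes a hardcoded limit, it ends the game and, after a short delay, destroys the session through GI_DefaultGameInstance.
; The end-game delegate only prints the resulting team.
; Team tickets are initialized in the construction script with increase and decrease functions, separate from the kill-based win check.
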(event Custom|OnEndGameWithResultDelegate_Event_0
  (params (TeamID :type E_TeamID%20Enum :default "GreenTeamID"))
  (Development|PrintString (Utilities|String|EnumtoString TeamID)))

(event EventBeginPlay
  (EventDispatchers|AssignOnEndGamewithResultDelegate (delegate Custom|OnEndGameWithResultDelegate_Event_0)))

(event EventTick
  (params (DeltaSeconds :type Float%20%28single-precision%29)))

(event EventAddKillforTeam
  (params (TeamID :type E_TeamID%20Enum :default "GreenTeamID"))
  ;[1 1 1] Its TDM GameMode
  (switch Utilities|FlowControl|Switch|SwitchonE_TeamID TeamID
    (:GreenTeamID
      (Class|TamSkadLecaTraceryGameModeBase|AddGreenTeamScore 1))
    (:RedTeamID
      (Class|TamSkadLecaTraceryGameModeBase|AddRedTeamScore 1)))
  (if (or (> (Math|Conversions|ToByte(Integer) (Class|TamSkadLecaTraceryGameModeBase|GetGreenTeamScore)) 5) (> (Math|Conversions|ToByte(Integer) (Class|TamSkadLecaTraceryGameModeBase|GetRedTeamScore)) 5))
    (Class|TeamDeathmatch|EndGamewithResult)
    (Development|PrintString "DESTROYING SESSION IN 5s")
    (Utilities|FlowControl|Delay 5.0)
    (bind _asgi_default_game_instance (Utilities|Casting|CastToGI_DefaultGameInstance (Game|GetGameInstance)))
    (Class|GameInstanceParent|DestroySession _asgi_default_game_instance)))

(fn ConstructionScript
  ;[1 1 1] set starting tickets
  (Variables|Default|SetGreenTeamTickets 10)
  (Variables|Default|SetRedTeamTickets 10))

(fn IncreaseTickets
  (params (IncreaseAmount :type Integer) (Team :type Integer))
  (switch int Team
    (:0
      ;[1 1 1] green alias  0
      (Variables|Default|SetGreenTeamTickets (+ (Variables|Default|GetGreenTeamTickets) IncreaseAmount)))
    (:1
      ;[1 1 1] red alias 1
      (Variables|Default|SetRedTeamTickets (+ (Variables|Default|GetRedTeamTickets) IncreaseAmount)))))

(fn DecreaseTickets
  (params (DecreaseAmount :type Integer) (Team :type Integer))
  (switch int Team
    (:0
      ;[1 1 1] green alias  0
      (Variables|Default|SetGreenTeamTickets (- (Variables|Default|GetGreenTeamTickets) DecreaseAmount)))
    (:1
      ;[1 1 1] red alias 1
      (Variables|Default|SetRedTeamTickets (- (Variables|Default|GetRedTeamTickets) DecreaseAmount)))))