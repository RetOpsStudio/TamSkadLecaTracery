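; Default AI character that carries a gun as a child actor and can switch between walk and jog speeds.
; BeginPlay caches the AI anim instance and gun references.
; Tick smoothly interpolates the capsule's yaw toward control rotation as a placeholder for turning.
; Fire and stop-fire events forward to the gun, with a delayed reload when it is not ready, pending a reload animation.
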(event Custom|Fire_Event
  (bind _gunreference (Variables|Default|GetGunReference))
  ;[1 1 1] gun manage
  (Default|FireEvent _gunreference)
  ;[1 1 1] animation isnt set yet
  (if (not (Class|GunParentV2|IsReadytoFire _gunreference))
    (Utilities|FlowControl|Delay 2.0)
    (Class|GunParentV2|Reload _gunreference)))

(event Custom|StopFire_Event
  ;[1 1 1] gun manage
  (Default|StopFireEvent (Variables|Default|GetGunReference)))

(event EventBeginPlay
  (bind _gun (Variables|Default|GetGun))
  (bind _childactor (Variables|/Script/Engine.ChildActorComponent|GetChildActor _gun))
  (bind (_asbp_gun_base _bsuccess) (Utilities|Casting|CastToBP_GunBase _childactor))
  (Variables|Default|SetABPAiReference (.AsABP%20AICharacter (Utilities|Casting|CastToABP_AICharacter (Components|SkeletalMesh|GetAnimInstance (Variables|Character|GetMesh)))))
  (Variables|Default|SetGunReference _asbp_gun_base)
  (Development|PrintString "Hello" _bsuccess))

(event Collision|EventActorBeginOverlap
  (params (OtherActor :type Actor%20Object%20Reference)))

(event EventTick
  (params (DeltaSeconds :type Float%20%28single-precision%29))
  (bind _capsulecomponent (Variables|Default|GetCapsuleComponent))
  ;[1 1 1] Placeholder  Smothly rotate to match controller rotation
  (Transformation|SetWorldRotation _capsulecomponent (Math|Rotator|MakeRotator 0.0 0.0 (.yaw (Math|Interpolation|RInterpTo (Transformation|GetWorldRotation _capsulecomponent) (Pawn|GetControlRotation :!class /Script/Engine.Pawn) (Utilities|Time|GetWorldDeltaSeconds) 25.0))) false false))

(fn ConstructionScript)

(fn SetSpeedtoWalk
  (Variables|/Script/Engine.CharacterMovementComponent|SetMaxWalkSpeed (Variables|Character|GetCharacterMovement) (Variables|Default|GetWalkSpeed)))

(fn SetSpeedtoJog
  (Variables|/Script/Engine.CharacterMovementComponent|SetMaxWalkSpeed (Variables|Character|GetCharacterMovement) (Variables|Default|GetJogSpeed)))