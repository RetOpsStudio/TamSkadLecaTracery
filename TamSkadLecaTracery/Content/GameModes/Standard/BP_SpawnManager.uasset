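; BP_SpawnManager is the deathmatch spawn manager actor, handling spawn point highlighting and player pawn respawns.
; After a short delay on BeginPlay, it registers itself with GS_DeathMatch and caches all BP_SpawnPoint actors, retrying if the cast game state is invalid.
; Show and hide events toggle lights on the cached points.
; RequestRespawnNewPawn spawns and returns a BP_PlayerCH at a supplied transform, adjusting for collision but always spawning.
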(event Custom|Retry
  (Utilities|FlowControl|Delay 0.1)
  (bind _asgs_death_match (Utilities|Casting|CastToGS_DeathMatch (Game|GetGameState)))
  (Utilities|IsValid _asgs_death_match
    (:Is%20Valid
      (Variables|/Game/GameModes/Standard/GS_DeathMatch.GS_DeathMatch_C|SetSpawnManageReference _asgs_death_match self)
      (bind _outactors (Actor|GetAllActorsOfClass "/Game/BP_SpawnPoint.BP_SpawnPoint_C"))
      (Variables|Default|SetSpawnPoints _outactors))
    (:Is%20Not%20Valid
      (CallFunction|Retry)
      (Development|PrintString "SpawnManagerRetry"))))

(event Custom|EVENT_ShowSpawns
  ;[1 1 1] turn on light on spawns
  (for _array_element (Variables|Default|GetSpawnPoints)
    (Default|EVENTHighlightSpawn _array_element)))

(event Custom|EVENT_HideSpawns
  ;[1 1 1] turn off light on spawns
  (for _array_element (Variables|Default|GetSpawnPoints)
    (Default|EVENTTurnOffLight _array_element)))

(event EventBeginPlay
  (Utilities|FlowControl|Delay 0.1)
  (bind _asgs_death_match (Utilities|Casting|CastToGS_DeathMatch (Game|GetGameState)))
  (Utilities|IsValid _asgs_death_match
    (:Is%20Valid
      (Variables|/Game/GameModes/Standard/GS_DeathMatch.GS_DeathMatch_C|SetSpawnManageReference _asgs_death_match self)
      (bind _outactors (Actor|GetAllActorsOfClass "/Game/BP_SpawnPoint.BP_SpawnPoint_C"))
      (Variables|Default|SetSpawnPoints _outactors))
    (:Is%20Not%20Valid
      (CallFunction|Retry)
      (Development|PrintString "SpawnManagerRetry"))))

(event Collision|EventActorBeginOverlap
  (params (OtherActor :type Actor%20Object%20Reference)))

(event EventTick
  (params (DeltaSeconds :type Float%20%28single-precision%29)))

(fn ConstructionScript)

(fn RequestRespawnNewPawn
  (params (RespawnTransform :type Transform))
  (bind _returnvalue (Game|SpawnActorfromClass "/Game/Characters/Player/BP_PlayerCH.BP_PlayerCH_C" RespawnTransform "AdjustIfPossibleButAlwaysSpawn" 0 0))
  (return _returnvalue))