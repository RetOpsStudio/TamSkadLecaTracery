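; BP_GunBase is the base gun Blueprint, loading magazine, ammo, fire rate and reload values from a data table row named after its class.
; Fire_Event repeats on a looping timer for full auto, firing from the muzzle socket with sound, ejected shells and camera shake.
; The timer clears on stop, when not ready, or when blocked, with an empty click if carried ammo runs out.
; Mesh overlaps, ignoring players and bullets, block firing inside walls.
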(event OnComponentBeginOverlap(SkeletalMeshComponent)
  (params (OverlappedComponent :type Primitive%20Component%20Object%20Reference) (OtherActor :type Actor%20Object%20Reference) (OtherComp :type Primitive%20Component%20Object%20Reference) (OtherBodyIndex :type Integer) (bFromSweep :type Boolean) (SweepResult :type Hit%20Result%20Structure%20%28by%20ref%29))
  ;[1 1 1] checks if weapon isnt inside a wall
  (Utilities|Casting|CastToCH_PlayerCharacter OtherActor
    (:CastFailed
      (Utilities|Casting|CastToBP_Bullet OtherActor
        (:CastFailed
          (Variables|Default|Setb_CanFIre false)
          (bind _asch_player_character (Utilities|Casting|CastToCH_PlayerCharacter (Actor|GetParentActor)))
          (Default|UpdateFireStatus _asch_player_character))))))

(event OnComponentEndOverlap(SkeletalMeshComponent)
  (params (OverlappedComponent :type Primitive%20Component%20Object%20Reference) (OtherActor :type Actor%20Object%20Reference) (OtherComp :type Primitive%20Component%20Object%20Reference) (OtherBodyIndex :type Integer))
  ;[1 1 1] checks if weapon isnt inside a wall
  (Utilities|Casting|CastToCH_PlayerCharacter OtherActor
    (:CastFailed
      (Utilities|Casting|CastToBP_Bullet OtherActor
        (:CastFailed
          (Variables|Default|Setb_CanFIre true))))))

(event Custom|StopFire_Event
  (Utilities|Time|ClearandInvalidateTimerbyHandle (stale Custom|Fire_Event _returnvalue_3)))

(event Custom|Fire_Event
  (bind _skeletalmeshcomponent (Variables|Default|GetSkeletalMeshComponent))
  (bind _skeletalmeshcomponent_2 (Variables|Default|GetSkeletalMeshComponent))
  (bind _returnvalue (Transformation|GetSocketTransform _skeletalmeshcomponent "b_gun_shelleject" "RTS_World"))
  (bind _returnvalue_2 (Transformation|GetSocketTransform _skeletalmeshcomponent_2 "Bullet" "RTS_World"))
  ;[1 1 1] Set timer for full auto
  (if (Class|GunParentV2|IsReadytoFire)
    (bind _returnvalue_3 (Utilities|Time|SetTimerbyEvent (delegate Custom|Fire_Event) (Class|GunParentV2|GetShotsInterval) true))
    ;[1 1 1] checs if weapon isnt inside wall
    (if (Variables|Default|Getb_CanFIre)
      ;[1 1 1] play sound
      (Audio|PlaySoundatLocation "/Game/Guns/Sound/gunshot.gunshot" (.location _returnvalue_2) (.rotation _returnvalue_2) 1.0 1.0 0.0 "/Game/Guns/Sound/BP_GunShotAttenuation.BP_GunShotAttenuation" 0 0)
      (Class|GunParentV2|Fire (Math|Transform|MakeTransform (.location _returnvalue_2) (.rotation _returnvalue_2) (.scale _returnvalue_2)) "/Game/Guns/Particles/P_MuzzleFlash.P_MuzzleFlash" _skeletalmeshcomponent_2 (Variables|Default|GetPlayerControllerID) (Variables|Default|GetControllerRef))
      ;[1 1 1] spawn empty shells
      (bind _returnvalue_4 (Game|SpawnActorfromClass "/Game/Guns/Attachments/BP_Shell.BP_Shell_C" (Math|Transform|MakeTransform (.location _returnvalue) (Math|Rotator|MakeRotator 0.0 9e+01 (.yaw (.rotation _returnvalue))) (.scale _returnvalue)) "Undefined" 0 0))
      (Physics|AddForce (Variables|/Game/Guns/Attachments/BP_Shell.BP_Shell_C|GetRoot _returnvalue_4) (+ (* (Math|Vector|GetUpVector _skeletalmeshcomponent) 70) (* (Math|Vector|GetForwardVector _skeletalmeshcomponent) (* (Math|Random|RandomIntegerinRange 120 200) -1))) "None" false)
      ;[1 1 1] shakes every cameras nerby
      (Audio|Components|Audio|Play (Variables|Default|GetCameraShakeSource))
      (bind _asch_player_character (Utilities|Casting|CastToCH_PlayerCharacter (Actor|GetParentActor)))
      (Default|UpdateFireStatus _asch_player_character)
      (else
        (Utilities|Time|ClearandInvalidateTimerbyHandle _returnvalue_3 :!label _label)))
    (elif (<= (Variables|Default|GetCarryOnAmmo) 0)
      ;;[1 1 1] play "click" if no ammo
      (Audio|PlaySoundatLocation "/Game/Guns/Sound/EmptyGun.EmptyGun" (Transformation|GetWorldLocation (Variables|Default|GetSkeletalMeshComponent)) "0, 0, 0" 1.0 1.0 0.0 "/Game/Guns/Sound/BP_GunShotAttenuation.BP_GunShotAttenuation" 0 0)
      (goto _label)
      (else
        (goto _label)))))

(fn ConstructionScript
  (bind _returnvalue (Utilities|GetDataTableRow "/Game/Guns/DataTables/Table_GunValues.Table_GunValues" (Utilities|String|StringToName (Utilities|GetClassDisplayName (Utilities|GetClass self))))
    (:then
      (bind _output_get (Variables|Default|SetMagazineSize (.magazinesize _returnvalue)))
      (Variables|Default|SetInMagAmmo _output_get)
      (Variables|Default|SetCarryOnAmmo (.carryonammo _returnvalue))
      (Variables|Default|SetShootsPerMinute (.shootsperminute _returnvalue))
      (Variables|Default|SetReloadTime (.reloadtime _returnvalue)))))